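; BP_Door3 is a door actor that swings open by rotating its Door component in yaw toward 90 degrees.
; OpenDoor sets IsOpen and plays a timeline whose float track drives a Lerp for the rotation, with no closing logic.
; BeginPlay calls OpenDoor if IsOpen is already set, and the overlap event is empty.
; The construction script applies DoorMaterial to the Cube component.
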(event Custom|OpenDoor
  (Variables|Default|SetisOpen true)
  (bind _doorfloat (Timeline|Timeline PlayFromStart)
    (:Update
      (Transformation|SetRelativeRotation (Variables|Default|GetDoor) (Math|Rotator|MakeRotator 0.0 0.0 (Math|Float|Lerp _doorfloat 9e+01 _doorfloat)) false false))))

(event EventBeginPlay
  (if (Variables|Default|GetisOpen)
    (CallFunction|OpenDoor)))

(event Collision|EventActorBeginOverlap
  (params (OtherActor :type Actor%20Object%20Reference)))

(event EventTick
  (params (DeltaSeconds :type Float%20%28single-precision%29)))

(fn ConstructionScript
  (Rendering|Material|SetMaterial (Variables|Default|GetCube) 0 (Variables|Default|GetDoorMaterial)))