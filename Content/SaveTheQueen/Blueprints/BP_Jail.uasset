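; BP_Jail is a jail door actor that opens when a BP_Saw overlaps it, then notifies the Queen through JailOpenCallback.
; OpenDoor sets IsOpen and plays a timeline that rotates the static mesh on roll, using the timeline float as both Lerp start and alpha toward 90 degrees.
; A jail already flagged IsOpen plays the opening on BeginPlay without notifying the Queen.
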(event Custom|OpenDoor
  (Variables|Default|SetisOpen true)
  (bind _doorfloat (Timeline|Timeline PlayFromStart)
    (:Update
      (Transformation|SetRelativeRotation (Variables|Default|GetStaticMesh) (Math|Rotator|MakeRotator (Math|Float|Lerp _doorfloat 9e+01 _doorfloat) 0.0 0.0) false false))))

(event EventBeginPlay
  (if (Variables|Default|GetisOpen)
    (CallFunction|OpenDoor)))

(event Collision|EventActorBeginOverlap
  (params (OtherActor :type Actor%20Object%20Reference))
  (Utilities|Casting|CastToBP_Saw OtherActor)
  (if (not (Variables|Default|GetisOpen))
    (CallFunction|OpenDoor)
    (Default|JailOpenCallback (Variables|Default|GetQueen))))

(event EventTick
  (params (DeltaSeconds :type Float%20%28single-precision%29)))

(fn ConstructionScript)