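; PasswordLock is a lock actor in the SaveTheQueen VR game that checks whether a password is correct through its Letters collection.
; Its IsValid function returns true only when every element in Letters reports itself valid.
; Separately, a VRPawn beginning or ending overlap with the lock shows or hides that pawn's debug display.
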(event EventBeginPlay)

(event Collision|EventActorBeginOverlap
  (params (OtherActor :type Actor%20Object%20Reference))
  (bind _asvrpawn (Utilities|Casting|CastToVRPawn OtherActor))
  (Default|ShowDebug _asvrpawn))

(event EventTick
  (params (DeltaSeconds :type Float%20%28single-precision%29)))

(event Collision|EventActorEndOverlap
  (params (OtherActor :type Actor%20Object%20Reference))
  (bind _asvrpawn (Utilities|Casting|CastToVRPawn OtherActor))
  (Default|HideDebug _asvrpawn))

(fn ConstructionScript)

(fn IsValid
  (Variables|Default|SetAllValid true)
  (for _array_element (Variables|Default|GetLetters)
    (if (not (Variables|/Game/SaveTheQueen/Blueprints/PasswordLetter.PasswordLetter_C|GetIsValid _array_element))
      (Variables|Default|SetAllValid false)))
  (return (Variables|Default|GetAllValid)))