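; BP_MusicButton is a world actor with a widget-based button that plays an assigned sound.
; On BeginPlay it passes itself and its Number as label to its WDG_MusicButton widget and loads Sound into its audio component, which the PlaySound event plays.
; A VRPawn overlapping the actor toggles that pawn's debug display on and off.
; A timeline-driven cube rotation is present but never runs.
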(event Custom|PlaySound
  (Audio|Components|Audio|Play (Variables|Default|GetAudio) 0.0))

(event EventBeginPlay
  (bind _aswdg_music_button (Utilities|Casting|CastToWDG_MusicButton (UserInterface|GetWidget (Variables|Default|GetWidgetButton))))
  (Variables|/Game/SaveTheQueen/Blueprints/WDG_MusicButton.WDG_MusicButton_C|SetMusicButton _aswdg_music_button self)
  (Variables|/Game/SaveTheQueen/Blueprints/WDG_MusicButton.WDG_MusicButton_C|SetText _aswdg_music_button (Variables|Default|GetNumber))
  (Audio|Components|Audio|SetSound (Variables|Default|GetAudio) (Variables|Default|GetSound)))

(event EventTick
  (params (DeltaSeconds :type Float%20%28single-precision%29)))

(event Collision|EventActorEndOverlap
  (params (OtherActor :type Actor%20Object%20Reference))
  (bind _asvrpawn (Utilities|Casting|CastToVRPawn OtherActor))
  (Default|HideDebug _asvrpawn))

(event Collision|EventActorBeginOverlap
  (params (OtherActor :type Actor%20Object%20Reference))
  (bind _asvrpawn (Utilities|Casting|CastToVRPawn OtherActor))
  (Default|ShowDebug _asvrpawn))

(fn ConstructionScript)