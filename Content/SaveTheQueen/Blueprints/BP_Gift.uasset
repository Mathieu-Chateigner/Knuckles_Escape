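; BP_Gift is a Save The Queen reward pedestal that raises a pillar and then spawns a keycard.
; GiveGift fires only once, guarded by the Activated flag, and plays a timeline that drives the pillar's relative Z.
; When the timeline finishes, IsBlackCard selects a black or regular keycard, spawned at the pillar's XY and rotation with a fixed height.
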(event Custom|GiveGift
  (params (isBlackCard :type Boolean))
  (bind _pillar (Variables|Default|GetPillar))
  (bind _returnvalue (Transformation|GetWorldTransform _pillar))
  (bind _returnvalue_2 (Math|Transform|MakeTransform (Math|Vector|MakeVector (.x (.location _returnvalue)) (.y (.location _returnvalue)) 1e+02) (.rotation _returnvalue)))
  (if (not (Variables|Default|GetActivated))
    (Variables|Default|SetActivated true)
    (bind _pillarfloat (Timeline|Timeline PlayFromStart)
      (:Update
        (Transformation|SetRelativeLocation (Variables|Default|GetPillar) (Math|Vector|MakeVector 0.0 0.0 (Math|Float|Lerp _pillarfloat 85.0 _pillarfloat)) false false))
      (:Finished
        (if isBlackCard
          (Game|SpawnActorfromClass "/Game/SaveTheQueen/Blueprints/BP_KeyCardBlack.BP_KeyCardBlack_C" _returnvalue_2 "Undefined" "MultiplyWithRoot" 0 0)
          (else
            (Game|SpawnActorfromClass "/Game/SaveTheQueen/Blueprints/BP_KeyCard.BP_KeyCard_C" _returnvalue_2 "Undefined" "MultiplyWithRoot" 0 0)))
        (Development|PrintString "SPAWN KEYCARD")))))

(event EventBeginPlay)

(event Collision|EventActorBeginOverlap
  (params (OtherActor :type Actor%20Object%20Reference)))

(event EventTick
  (params (DeltaSeconds :type Float%20%28single-precision%29)))

(fn ConstructionScript)