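; PasswordLetter is an actor for one cycling letter, apparently part of a password puzzle, that changes when a VRPawn overlaps it.
; ChangeLetter advances a wrapping index through the Letters array, stores the current letter and pushes it to the WDG_Letter widget.
; A Timeline, restarted on each successful change, animates the Cube's relative roll.
; Debug prints report each overlap and letter.
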(event Custom|ChangeLetter
  (bind _result (Math|Integer|IncrementInt (Variables|Default|GetCurrentIndex))
    (:%20%20
      (bind _output_get (Variables|Default|SetCurrentIndex (Math|Integer|%(Integer) _result (Utilities|Array|Length (Variables|Default|GetLetters)))))
      (bind _output_get_2 (Variables|Default|SetCurrentLetter (Utilities|Array|Get(acopy) (Variables|Default|GetLetters) _output_get)))
      (Development|PrintString _output_get_2)
      (bind _aswdg_letter (Utilities|Casting|CastToWDG_Letter (UserInterface|GetWidget (Variables|Default|GetWidget))))
      (Variables|/Game/SaveTheQueen/Blueprints/WDG_Letter.WDG_Letter_C|SetText _aswdg_letter (Variables|Default|GetCurrentLetter))
      ;[1 1 1] Animate
      (bind _doorfloat (Timeline|Timeline PlayFromStart)
        (:Update
          (Transformation|SetRelativeRotation (Variables|Default|GetCube) (Math|Rotator|MakeRotator (Math|Float|Lerp _doorfloat 1.8e+02 _doorfloat) 0.0 0.0) false false))))))

(event EventBeginPlay)

(event Collision|EventActorBeginOverlap
  (params (OtherActor :type Actor%20Object%20Reference))
  (Utilities|Casting|CastToVRPawn OtherActor)
  (CallFunction|ChangeLetter)
  (Development|PrintString "Overlap"))

(event EventTick
  (params (DeltaSeconds :type Float%20%28single-precision%29)))

(fn ConstructionScript)