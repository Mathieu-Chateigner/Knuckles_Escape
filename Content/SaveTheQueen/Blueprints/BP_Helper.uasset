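; BP_Helper is an NPC guide actor that tells the player how to escape by finding the queen and hands out the first keypass.
; On BeginPlay it caches the WDG_Dialogue from its widget and shows a placeholder line.
; The first overlap by a VRPawn triggers a timed, delay-chained sequence of dialogue updates, guarded by a one-shot flag, then calls GiveGift on its Gift reference.
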(event EventBeginPlay
  (bind _aswdg_dialogue (Utilities|Casting|CastToWDG_Dialogue (UserInterface|GetWidget (Variables|Default|GetWidget))))
  (Variables|Default|SetWDGDialogue _aswdg_dialogue)
  (Default|UpdateText (Variables|Default|GetWDGDialogue) "..."))

(event Collision|EventActorBeginOverlap
  (params (OtherActor :type Actor%20Object%20Reference))
  (Development|PrintString (Utilities|String|ToString(Object) OtherActor))
  (Utilities|Casting|CastToVRPawn OtherActor)
  (if (not (Variables|Default|GetTalkedOnce))
    (Variables|Default|SetTalkedOnce true)
    (Default|UpdateText (Variables|Default|GetWDGDialogue) "Hey you !")
    (Utilities|FlowControl|Delay 2.0)
    (Default|UpdateText (Variables|Default|GetWDGDialogue) "The only way for you to escape here is to find the queen")
    (Utilities|FlowControl|Delay 5.0)
    (Default|UpdateText (Variables|Default|GetWDGDialogue) "Take your first keypass on my left and find the queen")
    (Default|GiveGift (Variables|Default|GetGift))))

(event EventTick
  (params (DeltaSeconds :type Float%20%28single-precision%29)))

(fn ConstructionScript)