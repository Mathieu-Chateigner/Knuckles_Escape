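; BP_Door is a keycard-operated door for the SaveTheQueen game that can also start open.
; When a BP_KeyCard overlaps the closed door, it destroys the card and calls OpenDoor, which BeginPlay also calls if IsOpen is set.
; OpenDoor sets IsOpen and plays a Timeline that moves the Cube along relative Z, with no closing logic.
; The construction script applies DoorMaterial to the Cube.
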(event Custom|OpenDoor
  (Variables|Default|SetisOpen true)
  (bind _doorfloat (Timeline|Timeline PlayFromStart)
    (:Update
      (Transformation|SetRelativeLocation (Variables|Default|GetCube) (Math|Vector|MakeVector 0.0 0.0 (Math|Float|Lerp _doorfloat 3e+02 _doorfloat)) false false))))

(event EventBeginPlay
  (if (Variables|Default|GetisOpen)
    (CallFunction|OpenDoor)))

(event Collision|EventActorBeginOverlap
  (params (OtherActor :type Actor%20Object%20Reference))
  (bind _asbp_key_card (Utilities|Casting|CastToBP_KeyCard OtherActor))
  (if (not (Variables|Default|GetisOpen))
    (Actor|DestroyActor _asbp_key_card)
    (CallFunction|OpenDoor)))

(event EventTick
  (params (DeltaSeconds :type Float%20%28single-precision%29)))

(fn ConstructionScript
  (Rendering|Material|SetMaterial (Variables|Default|GetCube) 0 (Variables|Default|GetDoorMaterial)))